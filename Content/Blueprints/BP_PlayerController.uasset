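; Player controller for a branching text-scenario game that advances dialogue on left mouse release and records which of five endings is reached.
; BeginPlay unpacks DT_FinalScenario11 into parallel arrays for text, events, branches and commands, indexed by MessageIndex.
; Each click either updates BP_Userinterface text and choice buttons or, on an End command, unlocks that ending in the GameInstance and shows its UI.
; The event-string parser for spawning KANBANs is unconnected.
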(event EventBeginPlay
  (Input|EnableInput self)
  (bind _outrownames (DataTable|GetDataTableRowNames "/Game/Scenario/DT_FinalScenario11.DT_FinalScenario11"))
  (for (_array_element _array_index) _outrownames
    (bind _returnvalue (Utilities|GetDataTableRow "/Game/Scenario/DT_FinalScenario11.DT_FinalScenario11" _array_element)
      (:then
        (Utilities|Array|SetArrayElem (Variables|Default|GetDispTextArray) _array_index (Utilities|Array|Get(acopy) (.text _returnvalue)) true)
        (Utilities|Array|SetArrayElem (Variables|Default|GetOutRowEventArray) _array_index (Utilities|Array|Get(acopy) (.event _returnvalue)) true)
        (Utilities|Array|SetArrayElem (Variables|Default|GetWhoIDArray) _array_index (Utilities|Array|Get(acopy) (.who_id _returnvalue)) true)
        (Utilities|Array|SetArrayElem (Variables|Default|GetOutRowBranch1Array) _array_index (Utilities|Array|Get(acopy) (.branch1 _returnvalue)) true)
        (Utilities|Array|SetArrayElem (Variables|Default|GetOutRowB1Array) _array_index (Utilities|Array|Get(acopy) (.b1 _returnvalue)) true)
        (Utilities|Array|SetArrayElem (Variables|Default|GetOutRowBranch2Array) _array_index (Utilities|Array|Get(acopy) (.branch2 _returnvalue)) true)
        (Utilities|Array|SetArrayElem (Variables|Default|GetOutRowB2Array) _array_index (Utilities|Array|Get(acopy) (.b2 _returnvalue)) true)
        (Utilities|Array|SetArrayElem (Variables|Default|GetOutRowBranch3Array) _array_index (Utilities|Array|Get(acopy) (.branch3 _returnvalue)) true)
        (Utilities|Array|SetArrayElem (Variables|Default|GetOutRowB3Array) _array_index (Utilities|Array|Get(acopy) (.b3 _returnvalue)) true)
        (Utilities|Array|SetArrayElem (Variables|Default|GetOutRowBranch4Array) _array_index (Utilities|Array|Get(acopy) (.branch4 _returnvalue)) true)
        (Utilities|Array|SetArrayElem (Variables|Default|GetOutRowB4Array) _array_index (Utilities|Array|Get(acopy) (.b4 _returnvalue)) true)
        (Utilities|Array|SetArrayElem (Variables|Default|GetCommandArray) _array_index (Utilities|Array|Get(acopy) (.command _returnvalue)) true)
        (if (or (Utilities|Enum|Equal(Enum) (Utilities|Array|Get(acopy) (Variables|Default|GetCommandReference) (Variables|Default|GetCommandReferenceIndex)) (Utilities|Array|Get(acopy) (.command _returnvalue))) false)
          (Utilities|Array|Add (Variables|Default|GetCommandIndex) (+ _array_index 1))
          (Variables|Default|SetCommandReferenceIndex (+ (Variables|Default|GetCommandReferenceIndex) 1)))
        (Utilities|Array|SetArrayElem (Variables|Default|GetImageID) (Utilities|Array|Get(acopy) (.imageid _returnvalue)) _array_index true)))))

(event Input|MouseEvents|LeftMouseButton
  (params (Key :type Key%20Structure :default "AnyKey"))
  (bind _gameinstance (Variables|Default|GetGameInstance))
  (bind _gameinstance_2 (Variables|Default|GetGameInstance))
  (bind _gameinstance_3 (Variables|Default|GetGameInstance))
  (bind _gameinstance_4 (Variables|Default|GetGameInstance))
  (bind _gameinstance_5 (Variables|Default|GetGameInstance))
  (:Released
    (bind _end (CallFunction|CheckEnd))
    (if _end
      (switch string (Utilities|Array|Get(acopy) (Variables|Default|GetCommandArray) (Variables|Default|GetMessageIndex))
        (:End0
          (Utilities|Array|SetArrayElem (Variables|/Game/Blueprints/BP_GameInstance.BP_GameInstance_C|GetCanWatchEnding _gameinstance) 0 true true)
          (Variables|/Game/Blueprints/BP_GameInstance.BP_GameInstance_C|SetClearEndingNumberBuf _gameinstance 0))
        (:End1
          (Utilities|Array|SetArrayElem (Variables|/Game/Blueprints/BP_GameInstance.BP_GameInstance_C|GetCanWatchEnding _gameinstance_2) 1 true true)
          (Variables|/Game/Blueprints/BP_GameInstance.BP_GameInstance_C|SetClearEndingNumberBuf _gameinstance_2 1))
        (:End2
          (Utilities|Array|SetArrayElem (Variables|/Game/Blueprints/BP_GameInstance.BP_GameInstance_C|GetCanWatchEnding _gameinstance_3) 2 true true)
          (Variables|/Game/Blueprints/BP_GameInstance.BP_GameInstance_C|SetClearEndingNumberBuf _gameinstance_3 2))
        (:End3
          (Utilities|Array|SetArrayElem (Variables|/Game/Blueprints/BP_GameInstance.BP_GameInstance_C|GetCanWatchEnding _gameinstance_4) 3 true true)
          (Variables|/Game/Blueprints/BP_GameInstance.BP_GameInstance_C|SetClearEndingNumberBuf _gameinstance_4 3))
        (:End4
          (Utilities|Array|SetArrayElem (Variables|/Game/Blueprints/BP_GameInstance.BP_GameInstance_C|GetCanWatchEnding _gameinstance_5) 4 true true)
          (Variables|/Game/Blueprints/BP_GameInstance.BP_GameInstance_C|SetClearEndingNumberBuf _gameinstance_5 4)))
      (bind _foundwidgets (Widget|GetAllWidgetsOfClass "/Game/Blueprints/UI/BP_Userinterface.BP_Userinterface_C" true))
      (Default|CanSeeTitleButton (Utilities|Array|Get(acopy) _foundwidgets))
      (Default|CanNotReturnButton (Utilities|Array|Get(acopy) _foundwidgets))
      (Default|EndingText (Utilities|Array|Get(acopy) _foundwidgets) (Variables|/Game/Blueprints/BP_GameInstance.BP_GameInstance_C|GetClearEndingNumberBuf (Variables|Default|GetGameInstance)))
      (else
        (Variables|Default|SetMessageIndex (Math|Integer|Clamp(Integer) (|({2175806D-4D9D-9514-7DAE-CF8942FB3268}+1)) 0 (Utilities|Array|Length (Variables|Default|GetDispTextArray))))
        ;[1 1 1] コメント
        (bind _foundwidgets_2 (Widget|GetAllWidgetsOfClass "/Game/Blueprints/UI/BP_Userinterface.BP_Userinterface_C" true))
        ;[1 1 1] 次のテキストセット
        (Default|NextText (Utilities|Array|Get(acopy) _foundwidgets_2))
        (CallFunction|ShowCommandMenu)))))

(fn ConstructionScript
  (bind _asbp_game_instance (Utilities|Casting|CastToBP_GameInstance (Game|GetGameInstance)))
  (Variables|Default|SetGameInstance _asbp_game_instance))

(fn ShowCommandMenu
  (bind _messageindex (Variables|Default|GetMessageIndex))
  (bind _outrowbranch4array (Variables|Default|GetOutRowBranch4Array))
  (bind _item (Utilities|Array|Get(acopy) _outrowbranch4array _messageindex))
  (bind _foundwidgets (Widget|GetAllWidgetsOfClass "/Game/Blueprints/UI/BP_Userinterface.BP_Userinterface_C" true))
  (if (Utilities|Enum|NotEqual(Enum) (Utilities|Array|Get(acopy) (Variables|Default|GetOutRowBranch1Array) (Variables|Default|GetMessageIndex)) "")
    (Rendering|Components|TextRender|SetText (Variables|/Game/Blueprints/UI/BP_Userinterface.BP_Userinterface_C|GetSentakusi1 (Utilities|Array|Get(acopy) _foundwidgets)) (Utilities|Text|ToText(String) (Utilities|Array|Get(acopy) (Variables|Default|GetOutRowBranch1Array) _messageindex)))
    (Rendering|Components|TextRender|SetText (Variables|/Game/Blueprints/UI/BP_Userinterface.BP_Userinterface_C|GetSentakusi2 (Utilities|Array|Get(acopy) _foundwidgets)) (Utilities|Text|ToText(String) (Utilities|Array|Get(acopy) (Variables|Default|GetOutRowBranch2Array) _messageindex)))
    (Rendering|Components|TextRender|SetText (Variables|/Game/Blueprints/UI/BP_Userinterface.BP_Userinterface_C|GetSentakusi3 (Utilities|Array|Get(acopy) _foundwidgets)) (Utilities|Text|ToText(String) (Utilities|Array|Get(acopy) (Variables|Default|GetOutRowBranch3Array) _messageindex)))
    (Rendering|Components|TextRender|SetText (Variables|/Game/Blueprints/UI/BP_Userinterface.BP_Userinterface_C|GetSentakusi4 (Utilities|Array|Get(acopy) _foundwidgets)) (Utilities|Text|ToText(String) _item))
    ;[1 1 1] 選択肢表示
    (Widget|SetVisibility (Variables|/Game/Blueprints/UI/BP_Userinterface.BP_Userinterface_C|GetSentakusi1B (Utilities|Array|Get(acopy) _foundwidgets)) "Visible")
    (Widget|SetVisibility (Variables|/Game/Blueprints/UI/BP_Userinterface.BP_Userinterface_C|GetSentakusi2B (Utilities|Array|Get(acopy) _foundwidgets)) "Visible")
    (Widget|SetVisibility (Variables|/Game/Blueprints/UI/BP_Userinterface.BP_Userinterface_C|GetSentakusi3B (Utilities|Array|Get(acopy) _foundwidgets)) "Visible")
    (if (not (Utilities|Enum|Equal(Enum) _item ""))
      (Widget|SetVisibility (Variables|/Game/Blueprints/UI/BP_Userinterface.BP_Userinterface_C|GetSentakusi4B (Utilities|Array|Get(acopy) _foundwidgets)) "Visible"))))

(fn CheckEnd
  (bind _messageindex (Variables|Default|GetMessageIndex))
  (bind _commandarray (Variables|Default|GetCommandArray))
  (bind _item (Utilities|Array|Get(acopy) _commandarray _messageindex))
  (return (Math|Boolean|ORBoolean (Utilities|Enum|Equal(Enum) _item "End0") (Utilities|Enum|Equal(Enum) _item "End1") (Utilities|Enum|Equal(Enum) _item "End2") (Utilities|Enum|Equal(Enum) _item "End3") (Utilities|Enum|Equal(Enum) _item "End4"))))